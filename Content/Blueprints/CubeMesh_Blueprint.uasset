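; Cube mesh actor that spawns a particle effect on start and periodically toggles its material.
; BeginPlay spawns the emitter at a fixed offset above the static mesh.
; Tick counts frames and every 60th frame calls ChangeMetrial, which uses a boolean flag to alternate slot 0 between a color-grid material and the cube material.
; The timing is frame-based, so the switch rate depends on framerate.
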(event Custom|ChangeMetrial
  (bind _staticmeshcomponent (Variables|Debug|GetStaticMeshComponent))
  (if (Variables|Default|GetNewVar_0)
    (Rendering|Material|SetMaterial _staticmeshcomponent 0 "/Game/StarterContent/Materials/M_ColorGrid_LowSpec.M_ColorGrid_LowSpec")
    (Variables|Default|SetNewVar_0 false)
    (else
      (Rendering|Material|SetMaterial _staticmeshcomponent 0 "/Game/Geometry/Meshes/CubeMaterial.CubeMaterial")
      (Variables|Default|SetNewVar_0 true))))

(event EventBeginPlay
  (Variables|Default|SetNewVar_0 true)
  (Effects|SpawnEmitteratLocation "/Game/NewParticleSystem.NewParticleSystem" (+ (Transformation|GetWorldLocation (Variables|Debug|GetStaticMeshComponent)) "0, 0,400.000000")))

(event Collision|EventActorBeginOverlap
  (params (OtherActor :type Actor%20Object%20Reference)))

(event EventTick
  (params (DeltaSeconds :type Float%20%28single-precision%29))
  (bind _output_get (Variables|Default|SetNewVar_1 (+ (Variables|Default|GetNewVar_1) 1)))
  (if (== _output_get 60)
    (Variables|Default|SetNewVar_1 0)
    (CallFunction|ChangeMetrial)))

(fn ConstructionScript)